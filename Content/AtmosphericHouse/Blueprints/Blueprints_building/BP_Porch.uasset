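; BP_Porch is a modular building Blueprint that places a selectable porch mesh in the level.
; Its construction script picks the static mesh from an array, indexed by the Porch selection.
; A RevertDefaultMaterials toggle restores each material slot to the mesh's default, then clears itself, acting like an editor button.
; It has no active runtime logic.
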(fn `UserConstructionScript`
  (locals (`Number Of Materials` :type Integer))
  (bind _porch_mesh (`self.Porch_mesh`))
  ;[1 1 1] Porch
  (`StaticMeshComponent.SetStaticMesh` (`self.Porch_mesh`) (`|GetArrayItem` (`self.Porch Meshes`) (`KismetMathLibrary.Conv_ByteToInt` (`self.Porch`))))
  ;[1 1 1] Revert Materials
  (if (`self.Revert Default Materials`)
    (bind _output_get (set `local.Number Of Materials` (`PrimitiveComponent.GetNumMaterials` _porch_mesh)))
    (for _index (range (+ _output_get 1))
      (`PrimitiveComponent.SetMaterial` _porch_mesh _index (`StaticMesh.GetMaterial` (`StaticMeshComponent.StaticMesh` _porch_mesh) _index)))
    (set `self.Revert Default Materials` false)))