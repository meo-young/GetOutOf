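; BP_Floor is a modular building piece that places a floor and an optional ceiling for the house.
; The construction script picks meshes from arrays indexed by the floor-size enum, destroying either component when it is switched off.
; Broken ceilings swap in damaged meshes per size, with variant enums for 3x3 and 6x6, and sit 300 units up.
; A self-resetting toggle restores the floor mesh's default materials.
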(fn `UserConstructionScript`
  (locals (`Number Of Materials` :type Integer))
  (bind _ceiling_mesh (`self.Ceiling_mesh`))
  (bind _floor_mesh (`self.Floor_mesh`))
  (bind _floor_mesh_2 (`self.Floor_mesh`))
  ;[1 1 1] Floor
  (if (`self.Floor`)
    (`StaticMeshComponent.SetStaticMesh` _floor_mesh_2 (`|GetArrayItem` (`self.Floor Meshes`) (`KismetMathLibrary.Conv_ByteToInt` (`self.Floors`))))
    (else
      (`ActorComponent.K2_DestroyComponent` _floor_mesh_2)))
  (if (`self.Add Ceiling`)
    ;[1 1 1] Ceiling
    (if (`self.Ceiling Broken?`)
      (switch `/Game/AtmosphericHouse/Enums/E_Floors` (`self.Floors`)
        (:`NewEnumerator19`
          (`StaticMeshComponent.SetStaticMesh` (`self.Ceiling_mesh`) (`|GetArrayItem` (`self.Ceiling Meshes`) (`KismetMathLibrary.Conv_ByteToInt` (`self.Floors`))) :!label _label))
        (:`NewEnumerator25`
          (goto _label))
        (:`NewEnumerator43`
          (switch `/Game/AtmosphericHouse/Enums/E_Ceiling_3x3_broken` (`self.Ceiling 3x3 Broken`) :!label _label_2
            (:`NewEnumerator19`
              (`StaticMeshComponent.SetStaticMesh` _ceiling_mesh "/Game/AtmosphericHouse/Meshes/Meshes_building/SM_Ceiling_3x3_broken_A.SM_Ceiling_3x3_broken_A"))
            (:`NewEnumerator25`
              (`StaticMeshComponent.SetStaticMesh` _ceiling_mesh "/Game/AtmosphericHouse/Meshes/Meshes_building/SM_Ceiling_3x3_broken_B.SM_Ceiling_3x3_broken_B"))
            (:`NewEnumerator54`
              (`StaticMeshComponent.SetStaticMesh` _ceiling_mesh "/Game/AtmosphericHouse/Meshes/Meshes_building/SM_Ceiling_3x3_broken_C.SM_Ceiling_3x3_broken_C"))))
        (:`NewEnumerator44`
          (goto _label_2))
        (:`NewEnumerator45`
          (goto _label_2))
        (:`NewEnumerator46`
          (`StaticMeshComponent.SetStaticMesh` _ceiling_mesh "/Game/AtmosphericHouse/Meshes/Meshes_building/SM_Ceiling_4x3_broken_A.SM_Ceiling_4x3_broken_A"))
        (:`NewEnumerator47`
          (`StaticMeshComponent.SetStaticMesh` _ceiling_mesh "/Game/AtmosphericHouse/Meshes/Meshes_building/SM_Ceiling_6x3_broken_A.SM_Ceiling_6x3_broken_A" :!label _label_3))
        (:`NewEnumerator48`
          (goto _label_3))
        (:`NewEnumerator49`
          (goto _label))
        (:`NewEnumerator50`
          (goto _label))
        (:`NewEnumerator51`
          (switch `/Game/AtmosphericHouse/Enums/E_Ceiling_6x6_broken` (`self.Ceiling 6x6 Broken`)
            (:`NewEnumerator19`
              (`StaticMeshComponent.SetStaticMesh` _ceiling_mesh "/Game/AtmosphericHouse/Meshes/Meshes_building/SM_Ceiling_6x6_broken_A.SM_Ceiling_6x6_broken_A"))
            (:`NewEnumerator25`
              (`StaticMeshComponent.SetStaticMesh` _ceiling_mesh "/Game/AtmosphericHouse/Meshes/Meshes_building/SM_Ceiling_6x6_broken_B.SM_Ceiling_6x6_broken_B")))))
      (else
        (goto _label)))
    (`SceneComponent.K2_SetRelativeLocation` (`self.Ceiling_mesh`) (0.0 0.0 300.0) false false)
    (else
      (`ActorComponent.K2_DestroyComponent` (`self.Ceiling_mesh`))))
  ;[1 1 1] Revert Materials
  (if (`self.Revert Default Materials`)
    (bind _output_get (set `local.Number Of Materials` (`PrimitiveComponent.GetNumMaterials` _floor_mesh)))
    (for _index (range (+ _output_get 1))
      (`PrimitiveComponent.SetMaterial` _floor_mesh _index (`StaticMesh.GetMaterial` (`StaticMeshComponent.StaticMesh` _floor_mesh) _index)))
    (set `self.Revert Default Materials` false)))