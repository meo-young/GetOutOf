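; Demo actor for the ProHUD V2 Horror pack that shows a primary notification when the player character walks into its trigger box.
; On overlap by ThirdPersonCharacter_H, it passes its NotiInfo to the HUD manager to create the notification.
; The construction script previews that notification on a material billboard, using a dynamic material fed the background icon's texture and color, plus emissive power and size.
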(event `self.Box.OnComponentBeginOverlap`
  (params (OverlappedComponent :type "PrimitiveComponent Object Reference") (OtherActor :type "Actor Object Reference") (OtherComp :type "PrimitiveComponent Object Reference") (OtherBodyIndex :type Integer) (bFromSweep :type Boolean) (SweepResult :type "HitResult Structure (by ref)"))
  (cast `/Game/ProHUDV2_Horror/DemoContent/DemoCharacter/ThirdPersonCharacter_H` OtherActor)
  (`/Game/ProHUDV2_Horror/Blueprints/Libraries/BPi_HUDManagerV2_H.CreatePrimaryNotification_H` (`/Game/ProHUDV2_Horror/Blueprints/Libraries/BP_PHV2_Functions_H.GetHUDManager_H`) (`self.NotiInfo`)))

(event `UpdateActor`
  (bind _size (`self.Size`))
  (bind (_icontexture _transform _iconcolor) (break `/Game/ProHUDV2_Horror/Blueprints/Structs/S_IconInfo2_H` (`.BackgroundIconInfo_15_42C322FC40D1F8B5D2456B8E00E07933` (break `/Game/ProHUDV2_Horror/Blueprints/Structs/S_PrimaryNotiInfo_H` (`self.NotiInfo`)))))
  (bind (_r _g _b) (break `LinearColor` _iconcolor))
  (bind _returnvalue (`KismetMaterialLibrary.CreateDynamicMaterialInstance` (`.Material` (break `MaterialSpriteElement` (`|GetArrayItem` (`MaterialBillboardComponent.Elements` (`self.MaterialBillboard`)))))))
  (set `self.DynamicMaterial` _returnvalue)
  (`MaterialInstanceDynamic.SetTextureParameterValue` (`self.DynamicMaterial`) "Texture" (cast `Texture` _icontexture :!pure true))
  (`MaterialInstanceDynamic.SetVectorParameterValue` (`self.DynamicMaterial`) "Color" (`KismetMathLibrary.MakeColor` _r _g _b))
  (`MaterialInstanceDynamic.SetScalarParameterValue` (`self.DynamicMaterial`) "EmissivePower" (`self.EmissivePower`))
  (`MaterialBillboardComponent.SetElements` (`self.MaterialBillboard`) (`|MakeArray` (make `MaterialSpriteElement` :`Material` (`self.DynamicMaterial`) :`BaseSizeX` _size :`BaseSizeY` _size))))

(fn `UserConstructionScript`
  (`self.UpdateActor`))