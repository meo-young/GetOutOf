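; BP_HitFeedback_Demo_H is a demo trigger actor from the ProHUD V2 Horror content that sets the hit feedback style on the player character.
; On Box overlap it copies its feedback type and V1 settings into ThirdPersonCharacter_H, then briefly shows a PointLight as confirmation.
; End overlap only casts the character, and a Switch macro for compass, minimap and world markers is not used by the event graph.
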(event `self.Box.OnComponentBeginOverlap`
  (params (OverlappedComponent :type "PrimitiveComponent Object Reference") (OtherActor :type "Actor Object Reference") (OtherComp :type "PrimitiveComponent Object Reference") (OtherBodyIndex :type Integer) (bFromSweep :type Boolean) (SweepResult :type "HitResult Structure (by ref)"))
  (bind _pointlight (`self.PointLight`))
  (bind _asthird_person_character_h (cast `/Game/ProHUDV2_Horror/DemoContent/DemoCharacter/ThirdPersonCharacter_H` OtherActor))
  (set `/Game/ProHUDV2_Horror/DemoContent/DemoCharacter/ThirdPersonCharacter_H.FeedbackType` (`self.FeedbackType`) _asthird_person_character_h)
  (set `/Game/ProHUDV2_Horror/DemoContent/DemoCharacter/ThirdPersonCharacter_H.V1` (`self.V1`) _asthird_person_character_h)
  (set `/Game/ProHUDV2_Horror/DemoContent/DemoCharacter/ThirdPersonCharacter_H.V1_FeedbackType` (`self.FeedbackV1`) _asthird_person_character_h)
  (`SceneComponent.SetVisibility` _pointlight true false)
  (`KismetSystemLibrary.Delay` 0.3)
  (`SceneComponent.SetVisibility` _pointlight false false))

(event `self.Box.OnComponentEndOverlap`
  (params (OverlappedComponent :type "PrimitiveComponent Object Reference") (OtherActor :type "Actor Object Reference") (OtherComp :type "PrimitiveComponent Object Reference") (OtherBodyIndex :type Integer))
  (cast `/Game/ProHUDV2_Horror/DemoContent/DemoCharacter/ThirdPersonCharacter_H` OtherActor))

(fn `UserConstructionScript`
  (locals (DynamicMaterial :type "MaterialInstanceDynamic Object Reference")))