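; Demo trigger actor for the ProHUDV2 Horror kit that shows a screen effect when the third-person character enters its box.
; An Index variable selects blackscreen, highlight or one of three pulsing damage variants, created through the HUD manager.
; Leaving the box removes blackscreen and damage effects, but the highlight's removal call is never executed.
; The construction script writes the Text variable to a text render label.
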(event `self.Box.OnComponentBeginOverlap`
  (params (OverlappedComponent :type "PrimitiveComponent Object Reference") (OtherActor :type "Actor Object Reference") (OtherComp :type "PrimitiveComponent Object Reference") (OtherBodyIndex :type Integer) (bFromSweep :type Boolean) (SweepResult :type "HitResult Structure (by ref)"))
  (cast `/Game/ProHUDV2_Horror/DemoContent/DemoCharacter/ThirdPersonCharacter_H` OtherActor)
  (switch `int` (`self.Index`)
    (:`0`
      (`/Game/ProHUDV2_Horror/Blueprints/Libraries/BPi_HUDManagerV2_H.CreateHUDFX_Blackscreen_H` (`/Game/ProHUDV2_Horror/Blueprints/Libraries/BP_PHV2_Functions_H.GetHUDManager_H`) 0.3))
    (:`1`
      (`/Game/ProHUDV2_Horror/Blueprints/Libraries/BPi_HUDManagerV2_H.CreateHUDFX_Highlight_H` (`/Game/ProHUDV2_Horror/Blueprints/Libraries/BP_PHV2_Functions_H.GetHUDManager_H`) 0.2 0.9 (struct :`R` 1.0 :`G` 1.0 :`B` 1.0 :`A` 0.2) (struct :`R` 1.0 :`G` 1.0 :`B` 1.0 :`A` 1.0)))
    (:`2`
      (`/Game/ProHUDV2_Horror/Blueprints/Libraries/BPi_HUDManagerV2_H.CreateHUDFX_Damage_H` (`/Game/ProHUDV2_Horror/Blueprints/Libraries/BP_PHV2_Functions_H.GetHUDManager_H`) (struct :`R` 1.0 :`A` 0.8) (struct :`R` 0.614583 :`A` 0.2) true (0.0 0.5) 0.4 0.8))
    (:`3`
      (`/Game/ProHUDV2_Horror/Blueprints/Libraries/BPi_HUDManagerV2_H.CreateHUDFX_Damage_H` (`/Game/ProHUDV2_Horror/Blueprints/Libraries/BP_PHV2_Functions_H.GetHUDManager_H`) (struct :`R` 1.0 :`A` 0.7) (struct :`R` 0.614583 :`A` 0.23) true (0.0 0.9) 0.3 0.6))
    (:`4`
      (`/Game/ProHUDV2_Horror/Blueprints/Libraries/BPi_HUDManagerV2_H.CreateHUDFX_Damage_H` (`/Game/ProHUDV2_Horror/Blueprints/Libraries/BP_PHV2_Functions_H.GetHUDManager_H`) (struct :`R` 1.0 :`A` 0.5) (struct :`R` 0.614583 :`A` 0.9) true (0.5 0.9) 0.3 0.6))))

(event `self.Box.OnComponentEndOverlap`
  (params (OverlappedComponent :type "PrimitiveComponent Object Reference") (OtherActor :type "Actor Object Reference") (OtherComp :type "PrimitiveComponent Object Reference") (OtherBodyIndex :type Integer))
  (cast `/Game/ProHUDV2_Horror/DemoContent/DemoCharacter/ThirdPersonCharacter_H` OtherActor)
  (switch `int` (`self.Index`)
    (:`0`
      (`/Game/ProHUDV2_Horror/Blueprints/Libraries/BPi_HUDManagerV2_H.RemoveHUDFX_BlackScreen_H` (`/Game/ProHUDV2_Horror/Blueprints/Libraries/BP_PHV2_Functions_H.GetHUDManager_H`) 0.6 false))
    (:`1`)
    (:`2`
      (`/Game/ProHUDV2_Horror/Blueprints/Libraries/BPi_HUDManagerV2_H.RemoveHUDFX_Damage_H` (`/Game/ProHUDV2_Horror/Blueprints/Libraries/BP_PHV2_Functions_H.GetHUDManager_H`) false :!label _label))
    (:`3`
      (goto _label))
    (:`4`
      (goto _label))))

(fn `UserConstructionScript`
  (`TextRenderComponent.K2_SetText` (`self.TextRender`) (`self.Text`)))