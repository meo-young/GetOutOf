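; BP_Door is a door gimmick actor with separate open and unlock animations, each driven by a timeline that adds a yaw offset to the rotation captured beforehand.
; Opening plays an initial sound, waits, plays the opening sound while swinging, then after a pause snaps back to the yaw saved at BeginPlay.
; Unlocking runs its own timeline with no sound or reset.
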(event `self.ReceiveBeginPlay`
  (bind (_returnvalue_roll _returnvalue_pitch _returnvalue_yaw) (`KismetMathLibrary.BreakRotator` (`self.K2_GetActorRotation`)))
  (set `self.OriginYawValue` _returnvalue_yaw))

(event `self.PlayDoorOpenAnimation`
  (bind (_returnvalue_roll _returnvalue_pitch _returnvalue_yaw) (`KismetMathLibrary.BreakRotator` (`self.K2_GetActorRotation`)))
  (`GameplayStatics.PlaySoundAtLocation` "/Game/_GetOutOf/Sound/Door/SC_DoorOpened.SC_DoorOpened" (`self.K2_GetActorLocation`) (struct) 1.0 1.0 0.0 null null null null)
  (`KismetSystemLibrary.Delay` 1.6)
  (set `self.AccumulatedYawValue` _returnvalue_yaw)
  (`GameplayStatics.PlaySoundAtLocation` "/Game/_GetOutOf/Sound/Door/SC_DoorOpen.SC_DoorOpen" (`self.K2_GetActorLocation`) (struct) 1.0 1.0 0.0 null null null null)
  (bind (_direction _value) (`Timeline|DoorAnimation` :!via `PlayFromStart`)
    (:`Update`
      (`self.K2_SetActorRotation` (`KismetMathLibrary.MakeRotator` 0.0 0.0 (+ _value (`self.AccumulatedYawValue`)))))
    (:`Finished`
      (`KismetSystemLibrary.Delay` 1.8)
      (`self.K2_SetActorRotation` (`KismetMathLibrary.MakeRotator` 0.0 0.0 (`self.OriginYawValue`))))))

(event `self.PlayDoorUnlockAnimation`
  (bind (_returnvalue_roll _returnvalue_pitch _returnvalue_yaw) (`KismetMathLibrary.BreakRotator` (`self.K2_GetActorRotation`)))
  (set `self.AccumulatedYawValue` _returnvalue_yaw)
  (bind (_direction _value) (`Timeline|Timeline` :!via `PlayFromStart`)
    (:`Update`
      (`self.K2_SetActorRotation` (`KismetMathLibrary.MakeRotator` 0.0 0.0 (+ _value (`self.AccumulatedYawValue`)))))))

(fn `UserConstructionScript`)