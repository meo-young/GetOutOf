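; BP_TutorialGameModeBase is the tutorial game mode, handling the screen fade widget, a voice cue and horror effects.
; BeginPlay adds WBP_Fade and binds stage start to SameThing, which plays a delayed voice line, then unbinds.
; GetImperfecterActors caches Imperfecter Halation and NoiseGrain effects.
; SetHorrorEffects toggles them; enabling adds camera shake and a jumpscare sound, then automatically disables after a short delay.
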(event `self.ReceiveBeginPlay`
  (add `StageSubSystem.OnStageStartedDelegate` (subsystem `StageSubSystem`) (delegate `SameThing`))
  (bind _returnvalue (`|CreateWidget` "/Game/_GetOutOf/HUD/WBP_Fade.WBP_Fade_C" (`GameplayStatics.GetPlayerController` 0)))
  (`UserWidget.AddToViewport` _returnvalue 0)
  (set `self.FadeWidget` _returnvalue))

(event `SameThing`
  (`KismetSystemLibrary.Delay` 2.0)
  (`SoundSubSystem.PlayVoiceSFX` (subsystem `SoundSubSystem`) "SameThing" (`self.K2_GetActorLocation` (`GameplayStatics.GetPlayerPawn` 0)))
  (`KismetSystemLibrary.Delay` 2.0)
  (remove `StageSubSystem.OnStageStartedDelegate` (subsystem `StageSubSystem`) (delegate `SameThing`)))

(event `self.GetImperfecterActors`
  (bind _returnvalue (`ImperfecterSubsystem.GetImperfecterInstanceByID` (subsystem `ImperfecterSubsystem`) "IIA_0"))
  (bind _ashalation (cast `ImperfecterEffect_Halation` (`ImperfecterInstanceActor.GetImperfecterEffectByID` _returnvalue "Halation")))
  (set `self.As Halation` _ashalation)
  (bind _asnoise_grain (cast `ImperfecterEffect_NoiseGrain` (`ImperfecterInstanceActor.GetImperfecterEffectByID` _returnvalue "NoiseGrain")))
  (set `self.As Noise Grain` _asnoise_grain))

(event `self.SetHorrorEffects`
  (params (bEnable :type Boolean))
  (`/Engine/EditorBlueprintResources/StandardMacros.IsValid` (`self.As Halation`)
    (:`Is Valid`
      (set `ImperfecterEffect.bEnabled` bEnable (`self.As Halation`))
      (`/Engine/EditorBlueprintResources/StandardMacros.IsValid` (`self.As Noise Grain`)
        (:`Is Valid`
          (set `ImperfecterEffect.bEnabled` bEnable (`self.As Noise Grain`))
          (if bEnable
            (`PlayerCameraManager.StartCameraShake` :`self` (`GameplayStatics.GetPlayerCameraManager` 0) :`ShakeClass` "/Game/_GetOutOf/Blueprints/CameraShake/CSB_HorrorEffect.CSB_HorrorEffect_C")
            (`GameplayStatics.PlaySoundAtLocation` "/Game/All_In_One_HorrorGame_v1/Stereo/Jumpscare/Cue/Jumpscare_Behind_You_Stereo_Cue.Jumpscare_Behind_You_Stereo_Cue" (`self.K2_GetActorLocation` (`GameplayStatics.GetPlayerPawn` 0)) (struct) 1.0 1.0 0.0 null null null null)
            (`KismetSystemLibrary.Delay` 0.8)
            (`self.SetHorrorEffects` false)
            (else
              (`PlayerCameraManager.StopCameraShake` (`GameplayStatics.GetPlayerCameraManager` 0) null true))))))))

(fn `UserConstructionScript`)