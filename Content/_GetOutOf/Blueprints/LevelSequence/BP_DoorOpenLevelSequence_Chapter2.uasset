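; Level sequence Blueprint for Chapter 2 that plays a door-opening sequence after a short delay.
; DoorOpen plays it unconditionally, while DoorOpenIfNotTutorial plays it only when the game mode reports this is not the first play time.
; BeginPlay is empty, and the bindings of these events to the tutorial manager's all-tutorials-end delegate and the player's interaction-ended delegate are disconnected, so neither binding runs here.
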(event `self.ReceiveBeginPlay`)

(event `DoorOpen`
  (`KismetSystemLibrary.Delay` 2.0)
  (`self.PlayLevelSequence`))

(event `DoorOpenIfNotTutorial`
  (bind _asgoogame_mode_base (cast `GOOGameModeBase` (`GameplayStatics.GetGameMode`)))
  (if (not (`GOOGameModeBase.bIsFirstPlayTime` _asgoogame_mode_base))
    (`KismetSystemLibrary.Delay` 2.0)
    (`self.PlayLevelSequence`)))

(fn `UserConstructionScript`)