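; BP_MusicBox is an interactable music box item that clears the current stage after it is used.
; On BeginPlay it binds a Sound event to the interaction-start delegate.
; When triggered, it waits briefly, then spawns an attached music sound and plays a one-shot animation on the music box component.
; After a second fixed delay, without waiting for playback to finish, it calls ClearStage on the stage subsystem.
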(event `self.ReceiveBeginPlay`
  (add `InteractableItem.OnInteractionStartDelegate` (delegate `Sound`)))

(event `Sound`
  (`KismetSystemLibrary.Delay` 3.0)
  (`GameplayStatics.SpawnSoundAttached` "/Game/_GetOutOf/Sound/MusicBox/SC_MusicBox.SC_MusicBox" (`self.Music box`) "None" (`self.K2_GetActorLocation`) (struct) "KeepWorldPosition" true 1.0 1.0 0.0 null null)
  (`SkeletalMeshComponent.PlayAnimation` (`self.Music box`) "/Game/_GetOutOf/Mesh/MusicBox/scene/SkeletalMeshes/AM_MusicBox.AM_MusicBox" false)
  (`KismetSystemLibrary.Delay` 3.0)
  (`StageSubSystem.ClearStage` (subsystem `StageSubSystem`)))

(fn `UserConstructionScript`)