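; BP_DollItem3 is an interactable doll item that starts the doll spawning sequence when the player interacts with it.
; On BeginPlay it binds to the interaction-start delegate, whose handler finds BP_DollSpawner via GetActorOfClass, calls StartSpawn and destroys the item.
; Separately, Tick accumulates time, prints a one-time "Hello" debug string after a few seconds, then disables its own ticking.
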(event `self.ReceiveBeginPlay`
  (add `self.OnInteractionStartDelegate` (delegate `CustomEvent`)))

(event `CustomEvent`
  (bind _returnvalue (`GameplayStatics.GetActorOfClass` "/Game/_GetOutOf/Blueprints/Gimmic/BP_DollSpawner.BP_DollSpawner_C"))
  (`DollSpawner.StartSpawn` _returnvalue)
  (`self.K2_DestroyActor`))

(event `self.ReceiveTick`
  (params (DeltaSeconds :type "Float (single-precision)"))
  (bind _output_get (set `self.AccumulatedTime` (+ DeltaSeconds (`self.AccumulatedTime`))))
  (if (>= _output_get 5.0)
    (`/Engine/EditorBlueprintResources/StandardMacros.DoOnce` false
      (:`Completed`
        (`KismetSystemLibrary.PrintString` "Hello")
        (`self.SetActorTickEnabled` false)))))

(fn `UserConstructionScript`)