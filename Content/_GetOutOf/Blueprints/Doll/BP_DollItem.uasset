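; Interactable doll item that switches the level into its end-stage state and opens the way out.
; On BeginPlay it disables overlaps on the respawn trigger box, enables them on the end-stage trigger box and binds LightOn to interaction start.
; After a short delay, LightOn stops the BGM, plays the door-open level sequence and stops the light-off trigger's sequence.
; Level actors are found by class lookup, and a leftover debug print remains.
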(event `self.ReceiveBeginPlay`
  (bind _returnvalue (`GameplayStatics.GetActorOfClass` "/Game/_GetOutOf/Blueprints/Gimmic/BP_RespawnTriggerBox.BP_RespawnTriggerBox_C"))
  (set `PrimitiveComponent.bGenerateOverlapEvents` false (`TriggerBase.CollisionComponent` _returnvalue))
  (bind _returnvalue_2 (`GameplayStatics.GetActorOfClass` "/Game/_GetOutOf/Blueprints/Gimmic/BP_EndStageTriggerBox.BP_EndStageTriggerBox_C"))
  (set `PrimitiveComponent.bGenerateOverlapEvents` true (`TriggerBase.CollisionComponent` _returnvalue_2))
  (add `self.OnInteractionStartDelegate` (delegate `LightOn`))
  (`KismetSystemLibrary.PrintString` "Hello"))

(event `LightOn`
  (`KismetSystemLibrary.Delay` 1.5)
  (`SoundSubSystem.StopBGM` (subsystem `SoundSubSystem`))
  (bind _returnvalue (`GameplayStatics.GetActorOfClass` "/Game/_GetOutOf/Blueprints/LevelSequence/BP_DoorOpenLevelSequence.BP_DoorOpenLevelSequence_C"))
  (`GOOLevelSequenceActor.PlayLevelSequence` _returnvalue)
  (bind _returnvalue_2 (`GameplayStatics.GetActorOfClass` "/Game/_GetOutOf/Blueprints/LevelSequence/Stage/Chapter1/BP_4_LightOff_TriggerBox.BP_4_LightOff_TriggerBox_C"))
  (`GOOLevelSequenceActor.StopLevelSequence` _returnvalue_2))

(fn `UserConstructionScript`)