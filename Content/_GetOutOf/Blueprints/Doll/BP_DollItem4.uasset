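; BP_DollItem4 is an interactable doll item that completes the red-green light stage and can also stage a jump scare.
; Interaction clears the stage through the stage subsystem, finishes the game on BP_RedGreenLightManager, plays a voice SFX and destroys the doll.
; A separate ShowJumpScare event switches the player's view target to its camera's owner, triggers the game mode's jump scare and destroys the doll after a short delay.
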(event `self.ReceiveBeginPlay`
  (add `self.OnInteractionStartDelegate` (delegate `CustomEvent`)))

(event `CustomEvent`
  (`StageSubSystem.ClearStage` (subsystem `StageSubSystem`))
  (bind _returnvalue (`GameplayStatics.GetActorOfClass` "/Game/_GetOutOf/Blueprints/Gimmic/BP_RedGreenLightManager.BP_RedGreenLightManager_C"))
  (`RedGreenLightManager.FinishGame` _returnvalue)
  (`SoundSubSystem.PlayVoiceSFX` (subsystem `SoundSubSystem`) "BeingWith" (`self.K2_GetActorLocation`))
  (`self.K2_DestroyActor`))

(event `ShowJumpScare`
  (`PlayerController.SetViewTargetWithBlend` (`GameplayStatics.GetPlayerController` 0) (`ActorComponent.GetOwner` (`self.Camera`)) 0.0 "VTBlend_Linear" 0.0 false)
  (bind _asbp_game_mode_base (cast `/Game/_GetOutOf/Blueprints/Core/BP_GameModeBase` (`GameplayStatics.GetGameMode`)))
  (`/Game/_GetOutOf/Blueprints/Core/BP_GameModeBase.ShowJumpScare` _asbp_game_mode_base true)
  (`KismetSystemLibrary.Delay` 0.9)
  (`self.K2_DestroyActor`))

(fn `UserConstructionScript`)