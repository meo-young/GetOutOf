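; Actor component that displays its owner as an icon on the minimap.
; Shortly after BeginPlay it creates a WDG_MinimapIcon in the viewport and a helper SceneComponent attached to the player character's root.
; Each tick it moves the helper to the owner's world transform, then feeds its relative XY and yaw to the widget, getting player-relative placement through attachment.
; GetMapIconData exposes the owner's location, icon and size.
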(event `self.ReceiveBeginPlay`
  (`KismetSystemLibrary.Delay` 0.2)
  (bind _returnvalue (`|CreateWidget` "/Game/AdvancedMenu/BP/MinimapSystem/WDG_MinimapIcon.WDG_MinimapIcon_C"))
  (bind _output_get (set `self.Minimap Icon` _returnvalue))
  (`/Game/AdvancedMenu/BP/MinimapSystem/WDG_MinimapIcon.ChangeIcon` _output_get (`self.icon`))
  (`/Game/AdvancedMenu/BP/MinimapSystem/WDG_MinimapIcon.Change Size` _output_get (`self.icon size`))
  (`UserWidget.AddToViewport` _output_get 0)
  (bind _returnvalue_2 (`|AddComponentByClass` (`self.GetOwner`) "/Script/Engine.SceneComponent" false (`KismetMathLibrary.MakeTransform` (0.0 0.0 0.0))))
  (set `self.calc_helper` _returnvalue_2)
  (`SceneComponent.K2_AttachToComponent` (`self.calc_helper`) (`Actor.RootComponent` (`GameplayStatics.GetPlayerCharacter` 0)) "None" "KeepWorld" "KeepWorld" "KeepWorld" true))

(event `self.ReceiveTick`
  (params (DeltaSeconds :type "Float (single-precision)"))
  (`self.UpdateIconPosition`))

(fn `GetMapIconData`
  (returns (Location :type "Vector Structure") (Icon :type "Texture2D Object Reference") (`icon size` :type "Vector2D Structure"))
  (return (`Actor.K2_GetActorLocation` (`self.GetOwner`)) (`self.icon`) (`self.icon size`)))

(fn `UpdateIconPosition`
  (bind _returnvalue (`self.GetOwner`))
  (bind _calc_helper (`self.calc_helper`))
  (bind (_relativerotation_roll _relativerotation_pitch _relativerotation_yaw) (`KismetMathLibrary.BreakRotator` (`SceneComponent.RelativeRotation` _calc_helper)))
  (bind _calc_helper_2 (`self.calc_helper`)
    (:`then`
      (`SceneComponent.K2_SetWorldLocationAndRotation` _calc_helper_2 (`Actor.K2_GetActorLocation` _returnvalue) (`Actor.K2_GetActorRotation` _returnvalue) false false)
      (bind _minimap_icon (`self.Minimap Icon`)
        (:`then`
          (`/Game/AdvancedMenu/BP/MinimapSystem/WDG_MinimapIcon.UpdateIconLocation` _minimap_icon (`KismetMathLibrary.Conv_VectorToVector2D` (`SceneComponent.RelativeLocation` _calc_helper)) _relativerotation_yaw))
        (:`else`)))
    (:`else`)))