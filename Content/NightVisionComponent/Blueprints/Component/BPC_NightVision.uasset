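; Actor component that switches a night vision effect on or off on a supplied player camera through its post-process settings.
; InitializeNightVision forwards the requested state to ToggleNightVision, which has SetValues choose night vision or default exposure and film grain values and record the state.
; SetPostProcess then assigns the camera a newly built settings struct with those values and either the night vision or default post-process materials, replacing its previous settings.
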(fn `InitializeNightVision`
  (params (`Player Camera` :type "CameraComponent Object Reference") (On :type Boolean))
  (`self.ToggleNightVision` On `Player Camera`))

(fn `SetPostProcess`
  (params (`Player Camera` :type "CameraComponent Object Reference") (Index :type Boolean))
  (set `CameraComponent.PostProcessSettings` (make `PostProcessSettings` :`AutoExposureBias` (`self.Exposure Compensation`) :`FilmGrainIntensity` (`self.Film Grain Intensity`) :`FilmGrainTexelSize` (`self.Film Grain Texel Size`) :`WeightedBlendables` (select `bool` Index :`false` (`self.Default Material`) :`true` (`self.Night Vision Material`))) `Player Camera`))

(fn `SetValues`
  (params (On :type Boolean))
  (returns (Return :type Boolean))
  (if On
    (set `self.Exposure Compensation` (`self.Night Vision Exposure`))
    (set `self.Film Grain Intensity` (`self.Night Vision Grain Intensity`))
    (set `self.Film Grain Texel Size` (`self.Night Vision Grain Size`))
    (bind _output_get (set `self.NightVision?` true))
    (return _output_get)
    (else
      (set `self.Exposure Compensation` (`self.Default Exposure`))
      (set `self.Film Grain Intensity` (`self.Default Grain Intensity`))
      (set `self.Film Grain Texel Size` (`self.Default Grain Size`))
      (bind _output_get_2 (set `self.NightVision?` false))
      (return _output_get_2))))

(fn `ToggleNightVision`
  (params (On :type Boolean) (`Player Camera` :type "CameraComponent Object Reference"))
  (bind _return (`self.SetValues` On))
  (`self.SetPostProcess` `Player Camera` _return))